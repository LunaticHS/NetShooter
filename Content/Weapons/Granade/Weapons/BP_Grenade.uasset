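; BP_Grenade is a grenade actor that spawns a short-lived BP_Explosion at its own transform once armed by a brief delay after BeginPlay.
; Tick triggers the explosion at low speed, and Hit jumps into the same armed check for one class of hit actor.
; Hit also raises the mesh's linear damping on a class match.
; The graph never clears CanExplode or destroys the grenade, so explosions can spawn repeatedly.
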(event EventTick
  (params (DeltaSeconds :type Float%20%28single-precision%29))
  (if (< (Math|Vector|VectorLength (Transformation|GetVelocity)) 1e+02)
    (if (Variables|Default|GetCan%20Explode)
      (bind _returnvalue (Game|SpawnActorfromClass "/Game/Weapons/Granade/BP_Explosion.BP_Explosion_C" (Transformation|GetActorTransform) "Undefined" 0 0))
      (Actor|SetLifeSpan _returnvalue 3.0))))

(event Collision|EventHit
  (params (MyComp :type Primitive%20Component%20Object%20Reference) (Other :type Actor%20Object%20Reference) (OtherComp :type Primitive%20Component%20Object%20Reference) (bSelfMoved :type Boolean) (HitLocation :type Vector :default "0, 0, 0") (HitNormal :type Vector :default "0, 0, 0") (NormalImpulse :type Vector :default "0, 0, 0") (Hit :type Hit%20Result%20Structure%20%28by%20ref%29))
  (bind _returnvalue (Utilities|GetClass Other))
  (Utilities|FlowControl|Sequence
    (:then_0
      (if (== _returnvalue 0)
        (if (Variables|Default|GetCan%20Explode)
          (bind _returnvalue_2 (Game|SpawnActorfromClass "/Game/Weapons/Granade/BP_Explosion.BP_Explosion_C" (Transformation|GetActorTransform) "Undefined" 0 0))
          (Actor|SetLifeSpan _returnvalue_2 3.0))))
    (:then_1
      (if (== _returnvalue 0)
        (Class|PrimitiveComponent|SetLinearDamping (Variables|Default|GetStaticMesh self) 0.9)))))

(event EventBeginPlay
  (Utilities|FlowControl|Delay 0.7)
  (Variables|Default|SetCan%20Explode true))

(fn ConstructionScript)