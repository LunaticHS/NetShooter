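; Player state Blueprint that ends the game once a time limit of one minute has passed.
; Every tick it reads the current time from BP_GameState and, past the limit, pauses the game.
; A boolean flag, Condition, gates creation of the Over widget so it is added to the viewport only once.
; An unconnected debug print of the time remains in the graph.
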(event EventBeginPlay)

(event EventTick
  (params (DeltaSeconds :type Float%20%28single-precision%29))
  (bind _asbp_game_state (Utilities|Casting|CastToBP_GameState (Game|GetGameState)))
  (bind _returnvalue (Class|SGameState|Nowtime _asbp_game_state))
  (if (> _returnvalue 6e+01)
    (Game|SetGamePaused true)
    (if (Variables|Default|GetCondition)
      (bind _returnvalue_2 (UserInterface|CreateWidget "/Game/UI/Over.Over_C"))
      (UserInterface|Viewport|AddtoViewport _returnvalue_2 0)
      (Variables|Default|SetCondition false))))

(fn ConstructionScript)