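; Test game mode Blueprint that tracks kills and deaths through each player's SPlayerState.
; It binds to the OnActorKilled event on BeginPlay.
; Each kill adds a score point to the killer controller's pawn PlayerState, prints the total and copies it, truncated, to MyScore.
; A second sequence branch adds a death to the victim's SPlayerState when the victim is a PlayerPawn.
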(event Custom|OnActorKilled_Event_0
  (params (VictimActor :type Actor%20Object%20Reference) (KillerActor :type Actor%20Object%20Reference) (KillerController :type Controller%20Object%20Reference))
  (bind _returnvalue (Pawn|GetControlledPawn KillerController))
  (bind _playerstate (Variables|/Script/Engine.Pawn|GetPlayerState _returnvalue))
  (Utilities|FlowControl|Sequence
    (:then_0
      (if (Utilities|IsValid _playerstate)
        (bind _assplayer_state (Utilities|Casting|CastToSPlayerState _playerstate))
        (Class|SPlayerState|AddScore _assplayer_state 1.0)
        (Development|PrintString (Utilities|String|ToString(Float) (Variables|/Script/Engine.PlayerState|GetScore _assplayer_state)) true true "(R=0.124446,G=1.000000,B=0.000000,A=1.000000)")
        (Variables|Default|SetMyScore (Math|Float|Truncate (Variables|/Script/Engine.PlayerState|GetScore _assplayer_state)))))
    (:then_1
      (bind _asplayer_pawn (Utilities|Casting|CastToPlayerPawn VictimActor))
      (bind _assplayer_state_2 (Utilities|Casting|CastToSPlayerState (Variables|/Script/Engine.Pawn|GetPlayerState _asplayer_pawn)))
      (Class|SPlayerState|AddDeath _assplayer_state_2 1.0))))

(event EventBeginPlay
  (EventDispatchers|AssignOnActorKilled (delegate Custom|OnActorKilled_Event_0)))

(fn ConstructionScript)